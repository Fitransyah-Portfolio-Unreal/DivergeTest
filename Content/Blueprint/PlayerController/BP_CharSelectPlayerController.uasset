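; Player controller for a character select screen, with a base character step and a top customization step.
; BeginPlay creates both menu widgets, hides the second, and finds the tagged CharacterStorage placement actor.
; DisplaySelectedCharacter destroys the previous character, triggers the placement effect, spawns the selected class from the storage's map and saves the choice to the game instance.
; A step dispatcher shows the matching menu, filling the item grid from a data table.
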(event `self.ReceiveBeginPlay`
  (`|ExecutionSequence`
    (:`then_0`
      ;[1 1 1] Display First Widget
      (bind _returnvalue (`|CreateWidget` (`self.MenuDisplay_One`)))
      (bind _asmenu_display_one (cast `/Game/UI/MenuDisplay_One` _returnvalue))
      (bind _output_get (set `self.DisplayMenu_OneRef` _asmenu_display_one))
      (`UserWidget.AddToViewport` _output_get 0)
      (set `/Game/UI/MenuDisplay_One.PlayerController` self _output_get)
      (`WidgetBlueprintLibrary.SetInputMode_UIOnlyEx` self null "LockAlways")
      (set `self.bShowMouseCursor` true)
      (set `self.CurrentCharacterSelectStep` "NewEnumerator0"))
    (:`then_1`
      ;[1 1 1] Base Character Setup
      (bind _outactors (`GameplayStatics.GetAllActorsOfClassWithTag` "/Script/DivergeTest.CharacterStorage" "Placement"))
      (for _array_element _outactors
        (bind _ascharacter_storage (cast `CharacterStorage` _array_element))
        (bind _output_get_2 (set `self.As Character Storage` _ascharacter_storage))
        (bind _asplacement_actor (cast `/Game/Blueprint/Misc/PlacementActor` _output_get_2))
        (set `self.As Placement` _asplacement_actor)
        (`self.DisplaySelectedCharacter`)
        (set `/Game/UI/MenuDisplay_One.PlayerController` self (`self.DisplayMenu_OneRef`))
        ;[1 1 1] Costumization related event dispatcher
        (add `self.SelectStepDispatcher` (delegate `SelectStepDispatcher_Event`))))
    (:`then_2`
      ;[1 1 1] Display Second Widget and Hide it
      (bind _returnvalue_2 (`|CreateWidget` (`self.MenuDisplay_Two`)))
      (bind _asmenu_display_two (cast `/Game/UI/MenuDisplay_Two` _returnvalue_2))
      (bind _output_get_3 (set `self.Display Menu Two Ref` _asmenu_display_two))
      (`UserWidget.AddToViewport` _output_get_3 0)
      (`Widget.SetVisibility` _asmenu_display_two "Hidden")
      (set `/Game/UI/MenuDisplay_Two.PlayerController Ref` self _asmenu_display_two)
      ;[1 1 1] Game instance reference
      (bind _asbp_char_select_game_instance (cast `/Game/Blueprint/GameInstance/BP_CharSelectGameInstance` (`GameplayStatics.GetGameInstance`)))
      (set `self.As BP Char Select Game Instance` _asbp_char_select_game_instance))))

(event `SelectStepDispatcher_Event` :!signature `self.SelectStepDispatcher`
  (params (CurrentStep :type "/Game/Datas/Enum/CharacterSelectStep_Enum Enum" :default "NewEnumerator0"))
  ;[1 1 1] Costumization related event dispatcher
  (`self.SelecStepUpdated`))

(event `SelecStepUpdated`
  (bind _display_menu_two_ref (`self.Display Menu Two Ref`))
  ;[1 1 1] To do when player change back and fort (character select - costumization)
  (switch `/Game/Datas/Enum/CharacterSelectStep_Enum` (`self.CurrentCharacterSelectStep`)
    (:`NewEnumerator0`
      (`Widget.SetVisibility` (`self.DisplayMenu_OneRef`) "Visible"))
    (:`NewEnumerator1`
      (`Widget.SetVisibility` _display_menu_two_ref "Visible")
      (`PanelWidget.ClearChildren` (`/Game/UI/MenuDisplay_Two.ItemsGrid` _display_menu_two_ref))
      (`/Game/UI/MenuDisplay_Two.IterateByDataTable` _display_menu_two_ref "/Game/Datas/Table/CharacterTop_Table.CharacterTop_Table" "NewEnumerator1"))))

(event `On Character Updated`
  (bind _charcters (`self.Charcters`))
  ;[1 1 1] Destroy existing before spawn new
  (`/Engine/EditorBlueprintResources/StandardMacros.IsValid` _charcters
    (:`Is Valid`
      (`self.K2_DestroyActor` _charcters))))

(fn `DisplayFirstWidget`)

(fn `DisplaySelectedCharacter`
  (bind _displaymenu_oneref (`self.DisplayMenu_OneRef`))
  (bind _maincharmap (`CharacterStorage.MainCharMap` (`self.As Character Storage`)))
  (bind _returnvalue (`|GetEnumeratorNameAsString` (`/Game/UI/MenuDisplay_One.SelectedCharacter` _displaymenu_oneref)))
  (bind (_value _returnvalue_2) (`BlueprintMapLibrary.Map_Find` _maincharmap _returnvalue))
  ;[1 1 1] Event in player controller
  (`self.On Character Updated`)
  ;[1 1 1] Explosion
  (`/Game/Blueprint/Misc/PlacementActor.Emitting` (`self.As Placement`))
  ;[1 1 1] Spawn Base character based on enum in display one widget
  (`/Engine/EditorBlueprintResources/StandardMacros.IsValid` (`self.As Character Storage`)
    (:`Is Valid`
      (`/Engine/EditorBlueprintResources/StandardMacros.IsValid` _displaymenu_oneref
        (:`Is Valid`
          (if (`BlueprintMapLibrary.Map_Contains` _maincharmap _returnvalue)
            (if _returnvalue_2
              (bind _returnvalue_3 (`|SpawnActorFromClass` _value (`self.GetTransform` (`self.As Character Storage`)) "Undefined" "OverrideRootScale" null null))
              ;[1 1 1] Most updated character
              (set `self.Charcters` _returnvalue_3)
              (bind _asbp_char_select_game_instance (cast `/Game/Blueprint/GameInstance/BP_CharSelectGameInstance` (`GameplayStatics.GetGameInstance`)))
              (`/Game/Blueprint/GameInstance/BP_CharSelectGameInstance.SetSelectedCharacter` _asbp_char_select_game_instance (`/Game/UI/MenuDisplay_One.SelectedCharacter` (`self.DisplayMenu_OneRef`))))))))))

(fn `UserConstructionScript`)