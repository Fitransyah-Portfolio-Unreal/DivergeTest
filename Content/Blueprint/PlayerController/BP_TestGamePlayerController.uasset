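; Player controller for a gameplay (test) level that spawns the character picked in character selection and dresses it in the saved outfit.
; On BeginPlay it caches the game instance, sets game-only input and finds the tagged CharacterStorage actor.
; It looks up the selected class in that actor's map, spawns it there with customization marked finished, and possesses it.
; Saved top, bottom and feet row names are then sent through the fashion interface.
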(event `self.ReceiveBeginPlay`
  (bind _maincharmap (`CharacterStorage.MainCharMap` (`self.As Character Storage`)))
  (bind _returnvalue (`|GetEnumeratorNameAsString` (`/Game/Blueprint/GameInstance/BP_CharSelectGameInstance.SelectedCharacter` (`self.As BP Char Select Game Instance`))))
  (bind (_value _returnvalue_2) (`BlueprintMapLibrary.Map_Find` _maincharmap _returnvalue))
  (`|ExecutionSequence`
    (:`then_0`
      ;[1 1 1] Game instance Ref
      (bind _asbp_char_select_game_instance (cast `/Game/Blueprint/GameInstance/BP_CharSelectGameInstance` (`GameplayStatics.GetGameInstance`)))
      (set `self.As BP Char Select Game Instance` _asbp_char_select_game_instance)
      ;[1 1 1] Input mode
      (`WidgetBlueprintLibrary.SetInputMode_GameOnly` self)
      (set `self.bShowMouseCursor` false)
      ;[1 1 1] Charcter Storage Ref
      (bind _outactors (`GameplayStatics.GetAllActorsOfClassWithTag` "/Script/DivergeTest.CharacterStorage" "Pawn"))
      (if (> (`KismetArrayLibrary.Array_Length` _outactors) 0)
        (for _array_element _outactors
          (bind _ascharacter_storage (cast `CharacterStorage` _array_element))
          (set `self.As Character Storage` _ascharacter_storage))))
    (:`then_1`
      ;[1 1 1] Spawn and Posses Character
      (if (`BlueprintMapLibrary.Map_Contains` _maincharmap _returnvalue)
        (if _returnvalue_2
          (bind _returnvalue_3 (`|SpawnActorFromClass` _value (`self.GetTransform` (`self.As Character Storage`)) "Undefined" "OverrideRootScale" null null))
          (set `MainCharacter.bIsFinishCostumization` true _returnvalue_3)
          (`self.Possess` self _returnvalue_3)
          (set `self.MainCharacter Ref` _returnvalue_3))))
    (:`then_2`
      ;[1 1 1] Setup Fashion
      (if (`KismetSystemLibrary.DoesImplementInterface` (`self.MainCharacter Ref`) "/Game/Blueprint/Interface/BPI_FashionHelper.BPI_FashionHelper_C")
        (message `/Game/Blueprint/Interface/BPI_FashionHelper.SetupFashion` (`self.MainCharacter Ref`) "NewEnumerator1" (`/Game/Blueprint/GameInstance/BP_CharSelectGameInstance.TopRowName` (`self.As BP Char Select Game Instance`)))
        (message `/Game/Blueprint/Interface/BPI_FashionHelper.SetupFashion` (`self.MainCharacter Ref`) "NewEnumerator2" (`/Game/Blueprint/GameInstance/BP_CharSelectGameInstance.BottomRowName` (`self.As BP Char Select Game Instance`)))
        (message `/Game/Blueprint/Interface/BPI_FashionHelper.SetupFashion` (`self.MainCharacter Ref`) "NewEnumerator3" (`/Game/Blueprint/GameInstance/BP_CharSelectGameInstance.FeetRowName` (`self.As BP Char Select Game Instance`)))))))

(fn `UserConstructionScript`)